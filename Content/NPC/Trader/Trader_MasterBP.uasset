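; Master Blueprint for a trader NPC that highlights via custom depth when looked at and opens trade with the player character on interaction.
; It keeps a fixed-size slot inventory that stacks and spills items on add, takes across slots and compacts gaps.
; BPI functions expose items, slot info and a coin balance that cannot go negative.
; Slot and coin changes are pushed directly to the player's main menu widgets.
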(event EventBeginPlay
  (CallFunction|InvBeginPlay)
  (bind _aschar_bp (Utilities|Casting|CastToCharBP (Game|Player|GetPlayerPawn 0)))
  (bind _output_get (Variables|Default|SetAs%20Char%20BP _aschar_bp))
  (Utilities|FlowControl|Delay 0.2)
  (Variables|Default|SetMainMenuRef (Variables|/Game/BluePrints/CharBP.CharBP_C|GetMainMenuRef _output_get)))

(event Collision|EventActorBeginOverlap
  (params (OtherActor :type Actor%20Object%20Reference)))

(event EventTick
  (params (DeltaSeconds :type Float%20%28single-precision%29)))

(fn ConstructionScript)

(fn InvBeginPlay
  (Utilities|Array|Resize (Variables|Default|GetInv_SlotSkruckt) (Variables|Default|GetInv_MaxSlots)))

(fn InvGetSlotbyIndex
  (params (Index :type Integer))
  (bind _inv_slotskruckt (Variables|Default|GetInv_SlotSkruckt))
  (bind _output (Utilities|Array|Get(acopy) _inv_slotskruckt Index))
  (if (Utilities|IsValidClass (.item _output))
    (return false (Utilities|GetClassDefaults (.item _output)) (.amount _output) (.item _output))
    (else
      (return true "" 0 0))))

(fn InvFindEmptySlot
  (bind (_array_element _array_index) (Utilities|Array|ForEachLoopwithBreak (Variables|Default|GetInv_SlotSkruckt) :!label _label)
    (:LoopBody
      (if (not (Utilities|IsValidClass (.item _array_element)))
        (LocalVariables|SetSu true)
        (LocalVariables|SetInd _array_index)
        (goto _label Break)))
    (:Completed
      (return (LocalVariables|GetSu) (LocalVariables|GetInd)))))

(fn InvFindSlotforStuck
  (params (NewParam :type Item%20BP%20Master%20Class%20Reference))
  (bind (_array_element _array_index) (Utilities|Array|ForEachLoopwithBreak (Variables|Default|GetInv_SlotSkruckt) :!label _label)
    (:LoopBody
      (if (and (Utilities|IsValidClass (.item _array_element)) (== (.item _array_element) NewParam))
        (if (< (.amount _array_element) (.stuck (Utilities|GetClassDefaults (.item _array_element))))
          (LocalVariables|SetSu true)
          (LocalVariables|SetInd _array_index)
          (goto _label Break))))
    (:Completed
      (return (LocalVariables|GetSu) (LocalVariables|GetInd)))))

(fn InvUpdateWidgetSlot
  (params (Index :type Integer))
  (bind _mainmenuref (Variables|Default|GetMainMenuRef))
  (bind _traderslotsrefarray (Variables|/Game/Widhets/MenuUI.MenuUI_C|GetTraderSlotsRefArray _mainmenuref))
  (bind _output (Utilities|Array|Get(acopy) _traderslotsrefarray Index))
  (if (Utilities|IsValid _output)
    (Default|UpdateInfo _output)))

(fn InvAddItem
  (params (Item :type Item%20BP%20Master%20Class%20Reference) (Amount :type Integer))
  ;[1 1 1] Запись
  (Development|PrintString (Utilities|GetClassDisplayName Item))
  (LocalVariables|SetIt Item)
  (bind _output_get (LocalVariables|SetAm Amount))
  (if (>= _output_get 1)
    ;[1 1 1] Если предметов больше стака
    (bind _output_get_2 (LocalVariables|SetMaxStack (.Stuck (Utilities|Struct|BreakItemStruckt (Utilities|GetClassDefaults (LocalVariables|GetIt))))))
    (if (not (> (LocalVariables|GetAm) _output_get_2))
      _
      (else
        (LocalVariables|SetMoreThan2Stacks true)
        (LocalVariables|SetRestOfUnstack (LocalVariables|GetAm))))
    ;[1 1 1] Поиск слота для стака
    (bind (_succ _index) (CallFunction|InvFindSlotforStuck (LocalVariables|GetIt)))
    (if _succ
      (LocalVariables|SetSlot%20for%20Sack _index)
      ;[1 1 1] Помещается в ячейке?
      (bind _output_get_3 (LocalVariables|SetSummonItemsInStack (+ (LocalVariables|GetAm) (.amount (Utilities|Array|Get(acopy) (Variables|Default|GetInv_SlotSkruckt) (LocalVariables|GetSlot%20for%20Sack))))))
      (if (> _output_get_3 (LocalVariables|GetMaxStack))
        ;[1 0.4219 0.4219] Не поместилось
        (Utilities|Array|SetArrayElem (Variables|Default|GetInv_SlotSkruckt) (LocalVariables|GetSlot%20for%20Sack) (Utilities|Struct|MakeSlotStruckt (LocalVariables|GetIt) (LocalVariables|GetMaxStack)))
        (CallFunction|InvUpdateWidgetSlot (LocalVariables|GetSlot%20for%20Sack))
        (LocalVariables|SetRestOfUnstack (- (LocalVariables|GetSummonItemsInStack) (LocalVariables|GetMaxStack)))
        (LocalVariables|SetIsStack true)
        (else
          ;[0.7362 1 0.6537] Пометилось
          (Utilities|Array|SetArrayElem (Variables|Default|GetInv_SlotSkruckt) (LocalVariables|GetSlot%20for%20Sack) (Utilities|Struct|MakeSlotStruckt (LocalVariables|GetIt) (LocalVariables|GetSummonItemsInStack)))
          (CallFunction|InvUpdateWidgetSlot (LocalVariables|GetSlot%20for%20Sack))
          (Development|PrintString "Предмет застакан")
          (LocalVariables|SetIsStack true)
          (return true true 0))))
    ;[1 1 1] Добавление в новую ячейку
    (bind (_succ_2 _index_2) (CallFunction|InvFindEmptySlot :!label _label))
    (if _succ_2
      (LocalVariables|SetSlot%20for%20Sack _index_2)
      (if (LocalVariables|GetMoreThan2Stacks)
        (if (> (LocalVariables|GetRestOfUnstack) (LocalVariables|GetMaxStack))
          ;;[1 0.8806 0.41] Новый цикл
          (Utilities|Array|SetArrayElem (Variables|Default|GetInv_SlotSkruckt) (LocalVariables|GetSlot%20for%20Sack) (Utilities|Struct|MakeSlotStruckt (LocalVariables|GetIt) (LocalVariables|GetMaxStack)))
          (CallFunction|InvUpdateWidgetSlot (LocalVariables|GetSlot%20for%20Sack))
          (LocalVariables|SetRestOfUnstack (- (LocalVariables|GetRestOfUnstack) (LocalVariables|GetMaxStack)))
          (goto _label)
          (else
            (Utilities|Array|SetArrayElem (Variables|Default|GetInv_SlotSkruckt) (LocalVariables|GetSlot%20for%20Sack) (Utilities|Struct|MakeSlotStruckt (LocalVariables|GetIt) (LocalVariables|GetRestOfUnstack)))
            (CallFunction|InvUpdateWidgetSlot (LocalVariables|GetSlot%20for%20Sack))
            (LocalVariables|SetRestOfUnstack 0)
            (if (LocalVariables|GetIsStack)
              (Development|PrintString "Предметы застаканы + в новом слоте")
              (return true true 0)
              (else
                (Development|PrintString "Предметы добавлены в новый слот")
                (return true false 0)))))
        (else
          ;;[0.324 1 0] Поместилось сразу
          (Utilities|Array|SetArrayElem (Variables|Default|GetInv_SlotSkruckt) (LocalVariables|GetSlot%20for%20Sack) (Utilities|Struct|MakeSlotStruckt (LocalVariables|GetIt) (LocalVariables|GetAm)))
          (CallFunction|InvUpdateWidgetSlot (LocalVariables|GetSlot%20for%20Sack))
          (Development|PrintString "Предметы размещены в новом слоте")
          (return true false 0)))
      (else
        ;;[1 0 0] Инвентарь полон
        (Development|PrintString "Инентарь полонl")
        (if (LocalVariables|GetMoreThan2Stacks)
          (Development|PrintString (Utilities|String|ToString(Integer) (LocalVariables|GetRestOfUnstack)))
          (return false false (LocalVariables|GetRestOfUnstack))
          (else
            (return false false 0)))))
    (else
      ;[1 1 1] Попытка добавить <1 предмета
      (Development|PrintString "Попытка добавить <1 предмета")
      (return false false 0))))

(fn InvFindItem
  (params (LocClass :type Item%20BP%20Master%20Class%20Reference))
  (LocalVariables|SetClass LocClass)
  (LocalVariables|SetIndex (Utilities|Array|Length (Variables|Default|GetInv_SlotSkruckt)))
  (if (>= (LocalVariables|GetIndex) 0) :!label _label
    (if (== (.item (Utilities|Array|Get(acopy) (Variables|Default|GetInv_SlotSkruckt) (LocalVariables|GetIndex))) (LocalVariables|GetClass))
      (LocalVariables|SetIndex (LocalVariables|GetIndex))
      (LocalVariables|SetSLotAmount (.amount (Utilities|Array|Get(acopy) (Variables|Default|GetInv_SlotSkruckt) (LocalVariables|GetIndex))))
      (return true (LocalVariables|GetIndex) (LocalVariables|GetSLotAmount))
      (else
        (LocalVariables|SetIndex (- (LocalVariables|GetIndex) 1))
        (goto _label)))
    (else
      (return false 0 0))))

(fn InvRidOfEmptySlots
  (bind _inv_slotskruckt (Variables|Default|GetInv_SlotSkruckt))
  (if (<= (LocalVariables|GetIndex) (Utilities|Array|Length (Variables|Default|GetInv_SlotSkruckt))) :!label _label
    (if (== (.Item (Utilities|Struct|BreakSlotStruckt (Utilities|Array|Get(acopy) (Variables|Default|GetInv_SlotSkruckt) (LocalVariables|GetIndex)))) 0)
      (if (< (LocalVariables|GetFirstEmptySlot) 0)
        (LocalVariables|SetFirstEmptySlot (LocalVariables|GetIndex)))
      (elif (< (LocalVariables|GetFirstEmptySlot) 0)
        _
        (else
          (Utilities|Array|SetArrayElem _inv_slotskruckt (LocalVariables|GetFirstEmptySlot) (Utilities|Array|Get(acopy) _inv_slotskruckt (LocalVariables|GetIndex)))
          (CallFunction|InvUpdateWidgetSlot (LocalVariables|GetFirstEmptySlot))
          (Utilities|Array|SetArrayElem (Variables|Default|GetInv_SlotSkruckt) (LocalVariables|GetIndex) (Utilities|Struct|MakeSlotStruckt 0 0))
          (CallFunction|InvUpdateWidgetSlot (LocalVariables|GetIndex))
          (LocalVariables|SetIndex (LocalVariables|GetFirstEmptySlot))
          (LocalVariables|SetFirstEmptySlot -1)
          (goto _label))))
    (LocalVariables|SetIndex (+ (LocalVariables|GetIndex) 1))
    (goto _label)
    (else
      (return))))

(fn InvTakeItem
  (params (Class :type Item%20BP%20Master%20Class%20Reference) (Amount :type Integer))
  (LocalVariables|SetLocClass Class)
  (LocalVariables|SetLocAmount Amount)
  (if (.Suc (CallFunction|InvFindItem (LocalVariables|GetLocClass))) :!label _label
    (LocalVariables|SetIndex (.ID (CallFunction|InvFindItem (LocalVariables|GetLocClass))))
    (bind _output_get (LocalVariables|SetSlotAmount (.Amount (CallFunction|InvFindItem (LocalVariables|GetLocClass)))))
    (if (== (LocalVariables|GetLocAmount) _output_get)
      (Utilities|Array|SetArrayElem (Variables|Default|GetInv_SlotSkruckt) (LocalVariables|GetIndex) (Utilities|Struct|MakeSlotStruckt 0 0))
      (CallFunction|InvUpdateWidgetSlot (LocalVariables|GetIndex))
      (if (LocalVariables|GetIsFromOneSlot)
        (Development|PrintString "Предмет взят из 1 слота и опустошил его")
        (CallFunction|InvRidOfEmptySlots)
        (return true 0 true 0)
        (else
          (Development|PrintString "Предмет взят из нескольких слотов и опустошил последний")
          (CallFunction|InvRidOfEmptySlots)
          (return true 0 false (LocalVariables|GetLoops))))
      (elif (> (LocalVariables|GetLocAmount) _output_get)
        (LocalVariables|SetIsFromOneSlot false)
        (LocalVariables|SetLoops (+ (LocalVariables|GetLoops) 1))
        (Utilities|Array|SetArrayElem (Variables|Default|GetInv_SlotSkruckt) (LocalVariables|GetIndex) (Utilities|Struct|MakeSlotStruckt 0 0))
        (CallFunction|InvUpdateWidgetSlot (LocalVariables|GetIndex))
        (LocalVariables|SetLocAmount (- (LocalVariables|GetLocAmount) (LocalVariables|GetSlotAmount)))
        (goto _label)
        (else
          (Utilities|Array|SetArrayElem (Variables|Default|GetInv_SlotSkruckt) (LocalVariables|GetIndex) (Utilities|Struct|MakeSlotStruckt (LocalVariables|GetLocClass) (- (LocalVariables|GetSlotAmount) (LocalVariables|GetLocAmount))))
          (CallFunction|InvUpdateWidgetSlot (LocalVariables|GetIndex))
          (if (LocalVariables|GetIsFromOneSlot)
            (Development|PrintString "Предмет взят из 1 слота")
            (return true 0 true 0)
            (else
              (Development|PrintString "Предмет взят из нескольких слотов")
              (CallFunction|InvRidOfEmptySlots)
              (return true 0 false (LocalVariables|GetLoops)))))))
    (elif (LocalVariables|GetIsFromOneSlot)
      (Development|PrintString "Предмет не найден")
      (return false (LocalVariables|GetLocAmount) false 0)
      (else
        (Development|PrintString "Недостаточно предметов. Не забрано:")
        (Development|PrintString (Utilities|String|ToString(Integer) (LocalVariables|GetLocAmount)))
        (CallFunction|InvRidOfEmptySlots)
        (return false (LocalVariables|GetLocAmount) false 0)))))

(fn AddCoins
  (params (Amount :type Float%20%28single-precision%29))
  (if (>= (+ (Variables|Default|GetCoins) Amount) 0.0)
    (bind _output_get (Variables|Default|SetCoins (+ (Variables|Default|GetCoins) Amount)))
    (Rendering|Components|TextRender|SetText (Variables|/Game/Widhets/MenuUI.MenuUI_C|GetTraderMoney (Variables|Default|GetMainMenuRef)) (Utilities|Text|ToText(Float) _output_get "HalfToEven" false true 1 324 0 2))
    (return true)
    (else
      (return false))))

(fn BPIAddCoin
  (params (Amount :type Float%20%28single-precision%29))
  (bind _succ (CallFunction|AddCoins Amount))
  (return _succ))

(fn BPIAdditems
  (params (Item :type Item%20BP%20Master%20Class%20Reference) (Amount :type Integer))
  (Development|PrintString "Давай")
  (bind (_isadded _isstacked _itemsnotadded) (CallFunction|InvAddItem Item Amount))
  (return _isadded _isstacked _itemsnotadded))

(fn BPIGetSlotInfo
  (params (Index :type Integer))
  (bind (_empty _itemstruckt _amount _itemclass) (CallFunction|InvGetSlotbyIndex Index))
  (return _empty _itemstruckt _amount _itemclass))

(fn BPIGetTraderInfo
  (return (Variables|Default|GetInv_SlotSkruckt) (Variables|Default|GetCoins) false))

(fn BPITakeItems
  (params (Class :type Item%20BP%20Master%20Class%20Reference) (Amount :type Integer))
  (bind (_succ _items_not_taken) (CallFunction|InvTakeItem Class Amount))
  (return _succ _items_not_taken))

(fn EndLook
  (params (Actor :type Actor%20Object%20Reference))
  (Rendering|SetRenderCustomDepth (Variables|Character|GetMesh) false)
  (Development|PrintString "А куда")
  (return false))

(fn StartInterack
  (params (Actor :type Actor%20Object%20Reference))
  (Default|StartTrade (Variables|Default|GetAs%20Char%20BP) true self)
  (return false))

(fn StartLook
  (params (Actor :type Actor%20Object%20Reference))
  (Development|PrintString (Utilities|GetDisplayName self))
  (Rendering|SetRenderCustomDepth (Variables|Character|GetMesh) true)
  (return false))